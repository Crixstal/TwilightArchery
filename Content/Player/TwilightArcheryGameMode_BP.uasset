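; Game mode for a two-player boss fight that decides when the match is won or lost.
; On BeginPlay it finds both archer characters and the boss, then binds handlers to each Life death event.
; Game over requires both players dead, while boss death calls its OnDeath and leads to a win.
; Either outcome waits briefly, shows its widget with Retry focused, pauses the game and shows the cursor.
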(event `self.ReceiveBeginPlay`
  (`|ExecutionSequence`
    (:`then_0`
      (bind _outactors (`GameplayStatics.GetAllActorsOfClass` "/Game/Player/TwilightArcheryCharacter_BP.TwilightArcheryCharacter_BP_C"))
      (bind _output_get (set `self.playersArray` _outactors))
      (set `self.player1` (`|GetArrayItem` _output_get))
      (set `self.player2` (`|GetArrayItem` _output_get 1))
      (bind _returnvalue (`GameplayStatics.GetActorOfClass` "/Game/Enemy/BossCharacter_BP.BossCharacter_BP_C"))
      (set `self.Boss` _returnvalue))
    (:`then_1`
      (add `LifeComponent.deathEvent` (`TwilightArcheryCharacter.Life` (`self.player1`)) (delegate `Player1 dead`))
      (add `LifeComponent.deathEvent` (`TwilightArcheryCharacter.Life` (`self.player2`)) (delegate `Player2 dead`))
      (add `LifeComponent.deathEvent` (`BossCharacter.Life` (`self.Boss`)) (delegate `Boss dead`)))))

(event `Player1 dead`
  (set `self.1IsDead` true)
  (if (and (`self.1IsDead`) (`self.2IsDead`)) :!label _label
    (`KismetSystemLibrary.Delay` 3.0)
    (bind _returnvalue (`|CreateWidget` "/Game/Menus/GameOver.GameOver_C"))
    (`UserWidget.AddToViewport` _returnvalue 0)
    (`Widget.SetKeyboardFocus` (`/Game/Menus/GameOver.Retry` _returnvalue))
    (`GameplayStatics.SetGamePaused` true)
    (set `PlayerController.bShowMouseCursor` true (`GameplayStatics.GetPlayerController` 0))))

(event `Player2 dead`
  (set `self.2IsDead` true)
  (goto _label))

(event `Boss dead`
  (`BossCharacter.OnDeath` (`self.Boss`))
  (`KismetSystemLibrary.Delay` 3.0)
  (bind _returnvalue (`|CreateWidget` "/Game/Menus/Win.Win_C"))
  (`UserWidget.AddToViewport` _returnvalue 0)
  (`Widget.SetKeyboardFocus` (`/Game/Menus/Win.Retry` _returnvalue))
  (`GameplayStatics.SetGamePaused` true)
  (set `PlayerController.bShowMouseCursor` true (`GameplayStatics.GetPlayerController` 0)))

(fn `UserConstructionScript`)