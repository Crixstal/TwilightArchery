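; Player character Blueprint for the archer, handling bow feedback, movement sounds, death and ledge climbing.
; BowComponent delegates drive charge audio and effects, with Tick scaling particle spawn rate by charge time before a max-charge effect takes over.
; Hang snaps the capsule to traced wall points, and ClimbUp chains two MoveComponentTo moves, which hits interrupt.
; The trace-based ledge detection that calls Hang is currently disconnected.
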(event `self.BowComponent.startChargeDelegate`
  (bind _chargefx (`self.ChargeFX`))
  (`SceneComponent.SetHiddenInGame` _chargefx false false)
  (`ActorComponent.Activate` _chargefx false)
  (`NiagaraComponent.SetVariableFloat` _chargefx "SpawnRate" 1.0)
  (`AudioComponent.Play` (`self.BowAudio`) 0.0))

(event `self.ReceiveBeginPlay`
  (`NiagaraComponent.SetVariableFloat` (`self.ChargeFX`) "RadiusRotation" 4.0)
  (`NiagaraComponent.SetVariableFloat` (`self.ChargeFX`) "SpawnRate" 1.0)
  (`ActorComponent.Deactivate` (`self.ChargeFX`))
  (`ActorComponent.Deactivate` (`self.MaxChargeFX`))
  (set `CharacterMovementComponent.MaxWalkSpeed` (`self.baseWalkSpeed`) (`self.CharacterMovement`))
  (add `self.onHitEvent` (`|CreateDelegate` :!event `EventHit`))
  (add `self.jumpEvent` (`|CreateDelegate` :!event `OnJumpEvent`))
  (add `self.dodgeEvent` (`|CreateDelegate` :!event `OnDodgeEvent`))
  (add `LifeComponent.deathEvent` (`self.Life`) (`|CreateDelegate` :!event `OnDeathEvent`))
  (`AudioComponent.Stop` (`self.BowAudio`)))

(event `OnJumpEvent`
  (`GameplayStatics.PlaySoundAtLocation` "/Game/Sounds/Archer/Archer_Jump.Archer_Jump" (0.0 0.0 0.0) (struct) 0.2 1.0 0.0 null null null))

(event `self.BowComponent.shootDelegate`
  (bind _maxchargefx (`self.MaxChargeFX`))
  (`|ExecutionSequence`
    (:`then_0`
      (`SceneComponent.SetHiddenInGame` _maxchargefx false false)
      (`ActorComponent.Deactivate` _maxchargefx)
      (`AudioComponent.Stop` (`self.BowAudio`)))
    (:`then_1`
      (`GameplayStatics.PlaySoundAtLocation` "/Game/Sounds/Archer/Arrow/ArrowCue.ArrowCue" (0.0 0.0 0.0) (struct) 1.0 1.0 0.0 null null null))))

(event `self.BowComponent.chargeDelegate`)

(event `self.BowComponent.cancelChargeDelegate`
  (`AudioComponent.Stop` (`self.BowAudio`)))

(event `OnDodgeEvent`
  (`GameplayStatics.PlaySoundAtLocation` "/Game/Sounds/Archer/Dodge.Dodge" (0.0 0.0 0.0) (struct) 0.2 1.0 0.0 null null null))

(event `self.BowComponent.chargeMaxDelegate`
  (bind _chargefx (`self.ChargeFX`))
  (bind _maxchargefx (`self.MaxChargeFX`))
  (`|ExecutionSequence`
    (:`then_0`
      (`SceneComponent.SetHiddenInGame` _chargefx true false)
      (`ActorComponent.Deactivate` _chargefx))
    (:`then_1`
      (`SceneComponent.SetHiddenInGame` _maxchargefx false false)
      (`ActorComponent.Activate` _maxchargefx false)
      (`NiagaraComponent.ResetSystem` _maxchargefx)
      (`NiagaraComponent.SetVariableFloat` (`self.MaxChargeFX`) "RadiusRotation" 8.0)
      (`NiagaraComponent.SetVariableFloat` (`self.MaxChargeFX`) "SpawnRate" 70.0))
    (:`then_2`
      (`GameplayStatics.PlaySoundAtLocation` "/Game/Sounds/Archer/Arrow/MaxCharge.MaxCharge" (0.0 0.0 0.0) (struct) 0.1 0.6 0.0 null null null))))

(event `self.ReceiveTick`
  (params (DeltaSeconds :type "Float (single-precision)"))
  (bind _bowcomponent (`self.BowComponent`))
  (`|ExecutionSequence`
    (:`then_1`
      (if (`BowComponent.bIsCharging` _bowcomponent)
        (bind _returnvalue (`BowComponent.GetCurrentChargeTime` _bowcomponent))
        (bind _output_get (set `self.TimerAlpha` (/ _returnvalue (`BowComponent.maxChargeTime` _bowcomponent))))
        (`NiagaraComponent.SetVariableFloat` (`self.ChargeFX`) "SpawnRate" (`KismetMathLibrary.Lerp` 1.0 70.0 _output_get))))))

(event `OnDeathEvent`
  (bind _charactermovement (`self.CharacterMovement`))
  (set `self.bIsDead` true)
  (`CharacterMovementComponent.SetMovementMode` _charactermovement "MOVE_None" 0)
  (`MovementComponent.StopMovementImmediately` _charactermovement)
  (`PrimitiveComponent.SetCollisionEnabled` (`self.CapsuleComponent`) "NoCollision")
  (`GameplayStatics.PlaySoundAtLocation` "/Game/Sounds/Archer/PlayerDeath.PlayerDeath" (0.0 0.0 0.0) (struct) 0.7 1.0 0.0 null null null))

(event `InputAction|Test`
  (params (Key :type "Key Structure"))
  (:`Pressed`
    (if (`self.bIsClimbing`)
      (`self.OnHit` (0.0 1.0 0.0)))))

(event `InputAction|Test`
  (params (Key :type "Key Structure")))

(event `InputAction|ClimbUp`
  (params (Key :type "Key Structure"))
  ;[1 1 1] Climb Wall
  (:`Pressed`
    (if (`self.bIsClimbing`)
      (`self.ClimbUp`))))

(event `ClimbUp`
  (bind _capsulecomponent (`self.CapsuleComponent`))
  ;[1 1 1] Climb Wall
  (if (not (`self.IsClimbingUp`))
    (set `self.IsClimbingUp` true)
    (`KismetSystemLibrary.MoveComponentTo` _capsulecomponent (+ (`self.K2_GetActorLocation`) (0.0 0.0 145.0)) (`self.K2_GetActorRotation`) false false 0.8 :!label _label)
    (`KismetSystemLibrary.MoveComponentTo` _capsulecomponent (+ (`self.K2_GetActorLocation`) (* (`self.GetActorForwardVector`) 75.0) (0.0 0.0 15.0)) (`self.K2_GetActorRotation`) false false 0.6 :!label _label_2)
    (`self.ClimbEnd`)))

(event `ClimbEnd`
  (bind (_returnvalue_roll _returnvalue_pitch _returnvalue_yaw) (`KismetMathLibrary.BreakRotator` (`self.K2_GetActorRotation`)))
  (set `self.bIsClimbing` false)
  (`CharacterMovementComponent.SetMovementMode` (`self.CharacterMovement`) "MOVE_Walking" 0)
  (set `self.IsClimbingUp` false)
  (`self.K2_SetActorRotation` (`KismetMathLibrary.MakeRotator` _returnvalue_roll 0.0 _returnvalue_yaw)))

(event `EventHit`
  (`|ExecutionSequence`
    (:`then_0`
      (goto _label :!via `Stop`))
    (:`then_1`
      (goto _label_2 :!via `Stop`))
    (:`then_2`
      (`self.ClimbEnd`)
      (`GameplayStatics.PlaySoundAtLocation` "/Game/Sounds/Archer/Cough.Cough" (0.0 0.0 0.0) (struct) 0.4 1.0 0.0 null null null))))

(event `Hang`
  (bind _charactermovement (`self.CharacterMovement`))
  (bind (_heightlocation_x _heightlocation_y _heightlocation_z) (`KismetMathLibrary.BreakVector` (`self.HeightLocation`)))
  ;[1 1 1] Hanging
  (`CharacterMovementComponent.SetMovementMode` _charactermovement "MOVE_Flying" 0)
  (`MovementComponent.StopMovementImmediately` _charactermovement)
  (set `self.bIsClimbing` true)
  ;;[1 1 1] Replace correclty actor
  (`KismetSystemLibrary.MoveComponentTo` (`self.CapsuleComponent`) (`KismetMathLibrary.MakeVector` (.x (+ (* (`self.Wall Normal`) 30.0) (`self.Wall Location`))) (.y (+ (* (`self.Wall Normal`) 30.0) (`self.Wall Location`))) (- _heightlocation_z 75.0)) (`KismetMathLibrary.MakeRotFromX` (* (`self.Wall Normal`) -1.0)) true true))

(fn `ForwardTrace`
  (returns (ReturnValue :type Boolean))
  (bind _returnvalue (`self.K2_GetActorLocation`))
  (if (and (not (`self.bIsHit`)) (not (`self.bIsDodging`)) (not (`BowComponent.bIsAiming` (`self.BowComponent`))))
    (bind (_outhit _returnvalue_2) (`KismetSystemLibrary.SphereTraceSingle` :`Start` _returnvalue :`End` (+ _returnvalue (* (`self.GetActorForwardVector`) 150.0)) :`Radius` 10.0 :`TraceChannel` "TraceTypeQuery1" :`DrawDebugType` "ForOneFrame"))
    (set `self.Wall Normal` (`.Normal` (`GameplayStatics.BreakHitResult` _outhit)))
    (set `self.Wall Location` (`.Location` (`GameplayStatics.BreakHitResult` _outhit)))
    (return _returnvalue_2)))

(fn `HeightTrace`
  (params (InFrontOfAWall :type Boolean))
  (bind (_returnvalue_x _returnvalue_y _returnvalue_z) (`KismetMathLibrary.BreakVector` (`SceneComponent.GetSocketLocation` (`self.Mesh`) "HipsSocket")))
  (bind _returnvalue (+ (`self.K2_GetActorLocation`) (0.0 0.0 500.0) (* (`self.GetActorForwardVector`) 75.0)))
  (if InFrontOfAWall
    (bind (_outhit _returnvalue_2) (`KismetSystemLibrary.SphereTraceSingle` :`Start` _returnvalue :`End` (- _returnvalue (0.0 0.0 500.0)) :`Radius` 10.0 :`TraceChannel` "TraceTypeQuery1" :`DrawDebugType` "ForOneFrame"))
    (if _returnvalue_2
      (set `self.HeightLocation` (`.Location` (`GameplayStatics.BreakHitResult` _outhit)))
      (if (`KismetMathLibrary.InRange_FloatFloat` (- _returnvalue_z (.z (`.Location` (`GameplayStatics.BreakHitResult` _outhit)))) -50.0 0.0)
        (if (not (`self.bIsClimbing`))
          (`self.Hang`))))))

(fn `UserConstructionScript`)