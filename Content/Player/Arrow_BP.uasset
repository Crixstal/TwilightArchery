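; Arrow projectile actor that spins a Niagara effect in flight and destroys itself after a fixed lifetime.
; On BeginPlay it starts a timeline driving the effect's roll and binds to a hit delegate.
; On hit, the effect deactivates and an enemy or ground impact sound plays with randomized pitch.
; An unconnected branch for spawning a hit actor with the player's controller never runs.
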(event `OnComponentHit` :!signature `self.hitDelegate`
  (params (hasHitEnemy :type Boolean) (damage :type Integer))
  (bind _returnvalue (`KismetMathLibrary.RandomFloatInRange` 0.75 1.25))
  (bind _returnvalue_2 (`self.K2_GetActorLocation`))
  (`ActorComponent.Deactivate` (`self.Niagara`))
  (if hasHitEnemy
    (`GameplayStatics.PlaySoundAtLocation` "/Game/Sounds/Archer/Arrow/HitEnemy.HitEnemy" _returnvalue_2 (struct) 1.0 _returnvalue 0.0 null null null)
    (else
      (`GameplayStatics.PlaySoundAtLocation` "/Game/Sounds/Archer/Arrow/HitGround.HitGround" _returnvalue_2 (struct) 1.0 _returnvalue 0.0 null null null))))

(event `self.ReceiveBeginPlay`
  (`self.Rotate`)
  (add `self.hitDelegate` (delegate `OnComponentHit`))
  (`KismetSystemLibrary.Delay` 10.0)
  (`self.K2_DestroyActor`))

(event `Rotate`
  (`KismetSystemLibrary.PrintString` "Rotate")
  (bind (_direction _roll) (`Timeline|Rotation`)
    (:`Update`
      (`SceneComponent.K2_SetRelativeRotation` (`self.Niagara`) (`KismetMathLibrary.MakeRotator` _roll (.pitch (`SceneComponent.RelativeRotation` (`self.Niagara`))) (.yaw (`SceneComponent.RelativeRotation` (`self.Niagara`)))) false false))))

(fn `UserConstructionScript`)